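; Practice guard enemy Blueprint that patrols waypoints, spots the player and reflects its state through a visor material.
; FindTarget sphere-overlaps pawns within SightRadius and confirms line of sight to the player with a trace, while Tick draws that radius for debugging.
; GetTargetLocation and NextWaypoint supply a looping patrol route.
; Chase and lost-target events set the visor's Mood parameter; losing the target also stops movement and plays a look-around montage before signalling completion.
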(event `self.ReceiveBeginPlay`
  (bind _mesh (`self.Mesh`))
  (bind _returnvalue (`PrimitiveComponent.CreateDynamicMaterialInstance` _mesh 1 (`PrimitiveComponent.GetMaterial` _mesh 1) "None"))
  (set `self.MID_Visor` _returnvalue))

(event `self.ReceiveTick`
  (params (DeltaSeconds :type "Float (single-precision)"))
  (`parent.ReceiveTick` DeltaSeconds)
  (`KismetSystemLibrary.DrawDebugCircle` (`self.K2_GetActorLocation`) (`self.SightRadius`) 12 (struct :`R` 1.0 :`G` 1.0 :`B` 1.0 :`A` 1.0) 0.0 5.0 (`self.GetActorRightVector`) (`self.GetActorForwardVector`)))

(event `/Game/Blueprints/Test/13_BT/BPI_WaypointUser.NextWaypoint`
  (bind _result (`/Engine/EditorBlueprintResources/StandardMacros.IncrementInt` (`self.CurrentIndex`))
    (:`  `
      (set `self.CurrentIndex` (mod _result (`KismetArrayLibrary.Array_Length` (`self.Waypoints`)))))))

(event `/Game/Blueprints/Practice/0702/BPI_Chaser.OnLostTarget`
  (`Controller.StopMovement` (`self.GetController`))
  (`MaterialInstanceDynamic.SetScalarParameterValue` (`self.MID_Visor`) "Mood" (`self.LostEye`))
  (`|PlayMontage` (`self.Mesh`) (`self.LookAround`)
    (:`OnCompleted`
      (`MaterialInstanceDynamic.SetScalarParameterValue` (`self.MID_Visor`) "Mood" (`self.NormalEye`))
      (`self.OnLostTargetMontageEnd`))))

(event `/Game/Blueprints/Practice/0702/BPI_Chaser.OnChaseStart`
  (`MaterialInstanceDynamic.SetScalarParameterValue` (`self.MID_Visor`) "Mood" (`self.ChaseEye`)))

(event `/Game/Blueprints/Practice/0702/BPI_Chaser.OnChaseEnd`
  (`MaterialInstanceDynamic.SetScalarParameterValue` (`self.MID_Visor`) "Mood" (`self.NormalEye`)))

(fn `FindTarget`
  (returns (OutTarget :type "Actor Object Reference"))
  (locals (ReturnTarget :type "Actor Object Reference"))
  (bind _outactors (`KismetSystemLibrary.SphereOverlapActors` (`self.K2_GetActorLocation`) (`self.SightRadius`) (`|MakeArray` "ObjectTypeQuery3" :!type "EObjectTypeQuery Enum")))
  (for _array_element _outactors
    (if (== _array_element (`GameplayStatics.GetPlayerPawn` 0))
      (bind _outhit (`KismetSystemLibrary.LineTraceSingle` :`Start` (`self.K2_GetActorLocation`) :`End` (`self.K2_GetActorLocation` _array_element) :`TraceChannel` "TraceTypeQuery2" :`DrawDebugType` "ForOneFrame"))
      (if (== _array_element (`.HitActor` (`GameplayStatics.BreakHitResult` _outhit)))
        (set `local.ReturnTarget` _array_element)
        (break)
        (else
          (break)))))
  (return (`local.ReturnTarget`)))

(fn `GetTargetLocation`
  (returns (OutLocation :type "Vector Structure"))
  (bind _waypoints (`self.Waypoints`))
  (if (> (`KismetArrayLibrary.Array_Length` _waypoints) 0)
    (return (`self.K2_GetActorLocation` (`|GetArrayItem` _waypoints (`self.CurrentIndex`))))
    (else
      (return (0.0 0.0 0.0)))))

(fn `UserConstructionScript`
  (`parent.UserConstructionScript`))