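; Practice actor that bobs vertically above its spawn point in a smooth, looping motion.
; BeginPlay stores the start location, and Tick accumulates elapsed time.
; A cosine of that time, scaled to one full cycle per Duration and remapped to an inverted 0–1 range, is multiplied by MoveAmount as the Z offset.
; The inversion makes the motion start at the origin and ease in and out at both ends.
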(event `self.ReceiveBeginPlay`
  (set `self.StartLocation` (`self.K2_GetActorLocation`)))

(event `self.ReceiveTick`
  (params (DeltaSeconds :type "Float (single-precision)"))
  ; 시간 누적
  (bind _output_get (set `self.ElapsedTime` (+ DeltaSeconds (`self.ElapsedTime`))))
  ; 시작위치와 변화량을 더해서 새 위치 구하기
  (`self.K2_SetActorLocation` (+ (`KismetMathLibrary.MakeVector` 0.0 0.0 (* (- 1.0 (* (+ (`KismetMathLibrary.Cos` (/ (* _output_get (* (`KismetMathLibrary.GetPI`) 2.0)) (`self.Duration`))) 1.0) 0.5)) (`self.MoveAmount`))) (`self.StartLocation`))))

(fn `UserConstructionScript`
  (`parent.UserConstructionScript`))