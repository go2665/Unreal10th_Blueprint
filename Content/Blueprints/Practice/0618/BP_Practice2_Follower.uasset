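; BP_Practice2_Follower is a practice actor that follows the player pawn, which it caches on BeginPlay.
; Each Tick it moves at MoveSpeed along the normalized, height-flattened direction to the player, with no stopping distance.
; In the same update it eases its rotation toward that direction with RInterpTo, so turning lags behind movement.
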(event `self.ReceiveBeginPlay`
  (set `self.TargetPlayer` (`GameplayStatics.GetPlayerPawn` 0)))

(event `self.ReceiveTick`
  (params (DeltaSeconds :type "Float (single-precision)"))
  (bind _returnvalue (`KismetMathLibrary.MakeVector` (.x (- (`self.K2_GetActorLocation` (`self.TargetPlayer`)) (`self.K2_GetActorLocation`))) (.y (- (`self.K2_GetActorLocation` (`self.TargetPlayer`)) (`self.K2_GetActorLocation`)))))
  (`self.K2_SetActorLocationAndRotation` (+ (`self.K2_GetActorLocation`) (* DeltaSeconds (`self.MoveSpeed`) (`KismetMathLibrary.Normal` _returnvalue))) (`KismetMathLibrary.RInterpTo` (`self.K2_GetActorRotation`) (`KismetMathLibrary.Conv_VectorToRotator` _returnvalue) DeltaSeconds 1.0)))

(fn `UserConstructionScript`
  (`parent.UserConstructionScript`))