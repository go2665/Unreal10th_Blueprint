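; Practice actor that moves in a continuous loop through an array of waypoint actors at a set speed.
; Tick moves it along a cached direction without sweep and checks arrival by squared 2D distance against a squared radius.
; On arrival the index wraps by modulo, and the direction is recomputed on the XY plane, snapping the actor's rotation to face the next waypoint.
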(event `self.ReceiveBeginPlay`
  (`self.UpdateMoveDirection`))

(event `self.ReceiveTick`
  (params (DeltaSeconds :type "Float (single-precision)"))
  ; MoveDirection 방향으로 이동하기
  (`self.K2_SetActorLocation` (+ (`self.K2_GetActorLocation`) (* (`self.MoveDirection`) (`self.MoveSpeed`) DeltaSeconds)))
  (bind _returnvalue (`self.IsArrive`))
  (if _returnvalue
    (`self.IncreaseCurrent`)
    (`self.UpdateMoveDirection`)))

(fn `IsArrive`
  (returns (ReturnValue :type Boolean))
  (return (< (`KismetMathLibrary.Vector_Distance2DSquared` (`self.K2_GetActorLocation`) (`self.K2_GetActorLocation` (`|GetArrayItem` (`self.Waypoints`) (`self.CurrentIndex`)))) (`self.InRadiusSquared`))))

(fn `UserConstructionScript`
  (`parent.UserConstructionScript`))