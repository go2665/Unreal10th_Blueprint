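; BP_Practice03_SpinMove is a practice actor that travels in a straight line while spinning around the vertical axis.
; BeginPlay caches the actor's initial forward vector as MoveDirection, so the spin does not bend its path.
; Each Tick moves it along that direction by MoveSpeed and adds world yaw by SpinSpeed, both scaled by DeltaSeconds, without sweep collision.
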(event `self.ReceiveBeginPlay`
  (set `self.MoveDirection` (`self.GetActorForwardVector`)))

(event `self.ReceiveTick`
  (params (DeltaSeconds :type "Float (single-precision)"))
  ; MoveDirection 방향으로 이동하기
  (`self.K2_SetActorLocation` (+ (`self.K2_GetActorLocation`) (* (`self.MoveDirection`) (`self.MoveSpeed`) DeltaSeconds)))
  ; 초당 SpinSpeed각도 만큼 Yaw 회전
  (`self.K2_AddActorWorldRotation` (`KismetMathLibrary.MakeRotator` 0.0 0.0 (* (`self.SpinSpeed`) DeltaSeconds))))

(fn `UserConstructionScript`
  (`parent.UserConstructionScript`))