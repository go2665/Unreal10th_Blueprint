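; Practice actor that moves back and forth along its forward vector.
; Each Tick offsets its location by MoveSpeed, MoveDirection and delta time, without sweep, and accumulates ElapsedTime.
; Once ElapsedTime passes three seconds, MoveDirection flips sign and the timer resets.
; A DoOnce debug print announcing the three-second mark is left disconnected and never runs.
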(event `self.ReceiveBeginPlay`
  (set `self.ElapsedTime` 0.0)
  (set `self.MoveDirection` 1.0))

(event `self.ReceiveTick`
  (params (DeltaSeconds :type "Float (single-precision)"))
  (`self.K2_SetActorLocation` (+ (`self.K2_GetActorLocation`) (* (`self.GetActorForwardVector`) DeltaSeconds (`self.MoveSpeed`) (`self.MoveDirection`))))
  ; ElapsedTime(게임진행시간 누적하기)
  (bind _output_get (set `self.ElapsedTime` (+ DeltaSeconds (`self.ElapsedTime`))))
  ; ElapsedTime이 3초가 넘으면 이동방향을 뒤집고 ElapsedTime 초기화
  (if (> _output_get 3.0)
    (set `self.MoveDirection` (* (`self.MoveDirection`) -1.0))
    (set `self.ElapsedTime` 0.0)))

(fn `UserConstructionScript`)