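; BP_Enemy_BT3 is a test enemy, apparently for behavior tree use, that patrols waypoints and detects the player within a sight radius.
; FindTarget runs a sphere overlap on pawns and returns the player pawn if it is inside the radius.
; GetTargetLocation returns the current waypoint's location, or the origin when none exist, and NextWaypoint advances the index with wraparound.
; Tick draws the sight radius as a debug circle.
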(event `self.ReceiveTick`
  (params (DeltaSeconds :type "Float (single-precision)"))
  (`parent.ReceiveTick` DeltaSeconds)
  (`KismetSystemLibrary.DrawDebugCircle` (`self.K2_GetActorLocation`) (`self.SightRadius`) 12 (struct :`R` 1.0 :`G` 1.0 :`B` 1.0 :`A` 1.0) 0.0 5.0 (`self.GetActorRightVector`) (`self.GetActorForwardVector`)))

(event `self.NextWaypoint`
  (bind _result (`/Engine/EditorBlueprintResources/StandardMacros.IncrementInt` (`self.CurrentIndex`))
    (:`  `
      (set `self.CurrentIndex` (mod _result (`KismetArrayLibrary.Array_Length` (`self.Waypoints`)))))))

(fn `FindTarget`
  (returns (OutTarget :type "Actor Object Reference"))
  (locals (ReturnTarget :type "Actor Object Reference"))
  (bind _outactors (`KismetSystemLibrary.SphereOverlapActors` (`self.K2_GetActorLocation`) (`self.SightRadius`) (`|MakeArray` "ObjectTypeQuery3" :!type "EObjectTypeQuery Enum")))
  (for _array_element _outactors
    (if (== _array_element (`GameplayStatics.GetPlayerPawn` 0))
      (set `local.ReturnTarget` _array_element)
      (break)))
  (return (`local.ReturnTarget`)))

(fn `GetTargetLocation`
  (returns (OutLocation :type "Vector Structure"))
  (bind _waypoints (`self.Waypoints`))
  (if (> (`KismetArrayLibrary.Array_Length` _waypoints) 0)
    (return (`self.K2_GetActorLocation` (`|GetArrayItem` _waypoints (`self.CurrentIndex`))))
    (else
      (return (0.0 0.0 0.0)))))

(fn `UserConstructionScript`
  (`parent.UserConstructionScript`))